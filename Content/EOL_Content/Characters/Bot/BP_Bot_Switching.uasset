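; A controller Blueprint that lets the player switch possession between the BP_Bot characters in the level.
; On BeginPlay it gathers every BP_Bot into a roster and records the player's character as the current bot.
; Pressing B calls NextBot, which finds the current bot in the roster, advances to the following index with wraparound to the first, and possesses that bot.
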(event `self.ReceiveBeginPlay`
  (bind _outactors (`GameplayStatics.GetAllActorsOfClass` "/Game/EOL_Content/Characters/Bot/BP_Bot.BP_Bot_C"))
  (set `self.BotRoster` _outactors)
  (bind _asbp_bot (cast `/Game/EOL_Content/Characters/Bot/BP_Bot` (`GameplayStatics.GetPlayerCharacter` 0)))
  (set `self.CurrentBot` _asbp_bot))

(event `Key|B`
  (params (Key :type "Key Structure"))
  (:`Pressed`
    (`self.NextBot`)))

(fn `NextBot`
  (locals (LocalIndex :type Integer))
  (bind _returnvalue (`KismetArrayLibrary.Array_Find` (`self.BotRoster`) (`self.CurrentBot`)))
  (bind _returnvalue_2 (+ _returnvalue 1))
  (set `local.LocalIndex` _returnvalue)
  (bind _output_get (set `local.LocalIndex` (`KismetMathLibrary.SelectInt` _returnvalue_2 0 (`KismetArrayLibrary.Array_IsValidIndex` (`self.BotRoster`) _returnvalue_2))))
  (bind _output_get_2 (set `self.CurrentBot` (`|GetArrayItem` (`self.BotRoster`) _output_get)))
  (`self.Possess` _output_get_2))

(fn `UserConstructionScript`)