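; BP_SwitchDoor is a two-leaf door that opens while enough switches are active.
; SwitchActivated and SwitchDeactivated raise or lower an active-switch count, then compare it to the required number to play or reverse a timeline.
; The timeline lerps each leaf's relative location between its old and new positions, so a change in switch state can reverse the door mid-motion.
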(event `SwitchActivated`
  (`/Engine/EditorBlueprintResources/StandardMacros.IncrementInt` (`self.DoorSwitchesActive`)
    (:`  `
      (if (>= (`self.DoorSwitchesActive`) (`self.DoorSwitchesNeeded`))
        (bind (_direction _newtrack_01) (`Timeline|Timeline1` :!label _label)
          (:`Update`
            (`|ExecutionSequence`
              (:`then_0`
                (`SceneComponent.K2_SetRelativeLocation` (`self.DoorLeafR`) (`KismetMathLibrary.VLerp` (`self.RLeafOld`) (`self.RLeafNew`) _newtrack_01) false false))
              (:`then_1`
                (`SceneComponent.K2_SetRelativeLocation` (`self.DoorLeafL`) (`KismetMathLibrary.VLerp` (`self.LLeafOld`) (`self.LLeafNew`) _newtrack_01) false false)))))
        (else
          (goto _label :!via `Reverse`))))))

(event `SwitchDeactivated`
  (`/Engine/EditorBlueprintResources/StandardMacros.DecrementInt` (`self.DoorSwitchesActive`)
    (:`  `
      (if (>= (`self.DoorSwitchesActive`) (`self.DoorSwitchesNeeded`))
        (goto _label)
        (else
          (goto _label :!via `Reverse`))))))

(fn `UserConstructionScript`)